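; In-heist actor for a custom reticle mod that applies saved reticle materials and weapon data when a heist starts.
; On BeginPlay it reads BP_CustomReticlesPersistent and writes its materials straight into the mapped meshes' material slots, avoiding late secondary-material swaps.
; It polls until BP_CustomReticle exists, passes it the heist weapon array, then calls GetGun after a delay.
; An L-key toggle for the customiser widget is present but disconnected.
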(event EventBeginPlay
  ;[1 1 1] Get persisent obj
  (bind _objectinstance (CallFunction|FindPersistentModObjectbyClass "/Game/Mods/_TannerMod/LizReticle/BP_CustomReticlesPersistent.BP_CustomReticlesPersistent_C"))
  (bind _asbp_custom_reticles_persistent (Utilities|Casting|CastToBP_CustomReticlesPersistent _objectinstance))
  (Variables|Default|SetPersistent _asbp_custom_reticles_persistent)
  ;[1 1 1] Setup materials; Doing this to speedily set materials because going through the entire process of getting them and stuff is too slow and results in secondary material being set too late
  (bind _keys (Utilities|Map|Keys (Variables|/Game/Mods/_TannerMod/LizReticle/BP_CustomReticlesPersistent.BP_CustomReticlesPersistent_C|GetheistMeshMap (Variables|Default|GetPersistent))))
  (for _array_element _keys
    (bind _structout (Utilities|Struct|SetmembersinSkeletalMaterial (Utilities|Array|Get(acopy) (Variables|/Script/Engine.SkeletalMesh|GetMaterials _array_element) (.Value (Utilities|Map|Find (Variables|/Game/Mods/_TannerMod/LizReticle/BP_CustomReticlesPersistent.BP_CustomReticlesPersistent_C|GetheistMeshMap (Variables|Default|GetPersistent)) _array_element))) (.Value (Utilities|Map|Find (Variables|/Game/Mods/_TannerMod/LizReticle/BP_CustomReticlesPersistent.BP_CustomReticlesPersistent_C|GetheistMaterialMap (Variables|Default|GetPersistent)) (.Value (Utilities|Map|Find (Variables|/Game/Mods/_TannerMod/LizReticle/BP_CustomReticlesPersistent.BP_CustomReticlesPersistent_C|GetheistMeshMap (Variables|Default|GetPersistent)) _array_element))))))
    (Utilities|Array|SetArrayElem (Variables|/Script/Engine.SkeletalMesh|GetMaterials _array_element) (.Value (Utilities|Map|Find (Variables|/Game/Mods/_TannerMod/LizReticle/BP_CustomReticlesPersistent.BP_CustomReticlesPersistent_C|GetheistMeshMap (Variables|Default|GetPersistent)) _array_element)) _structout))
  (bind _outactors (Actor|GetAllActorsOfClass "/Game/Mods/_TannerMod/LizReticle/BP_CustomReticle.BP_CustomReticle_C" :!label _label))
  (if (== (Utilities|Array|Get(acopy) _outactors) 0)
    (Utilities|FlowControl|Delay 0.2)
    (goto _label)
    (else
      (Variables|Default|SetMainBP (Utilities|Array|Get(acopy) _outactors))
      ;[1 1 1] Nessecary setup
      (Variables|/Game/Mods/_TannerMod/LizReticle/BP_CustomReticle.BP_CustomReticle_C|SetWeaponArray (Variables|Default|GetMainBP) (Variables|/Game/Mods/_TannerMod/LizReticle/BP_CustomReticlesPersistent.BP_CustomReticlesPersistent_C|GetheistWeaponArray (Variables|Default|GetPersistent)))
      (Utilities|FlowControl|Delay 2.0)
      (Default|GetGun (Variables|Default|GetMainBP)))))

(fn ConstructionScript
  (|CallParentFunction))