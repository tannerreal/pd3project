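; Mod actor that spawns a custom assault banner when the heist action phase begins, plus a key-toggled settings widget for it.
; Banner position, scale and settings key load from the VoidSave slot, while slider previews update the banner without saving.
; An Asset Registry folder scan maps music AkEvents to BPM data.
; Blink speed follows the Heist Jukebox or world-settings track, unless saved debug values override it.
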(event Custom|eventVoidBannerUpdate
  (bind _jukeboxpersistent (Variables|Default|GetJukeboxPersistent))
  (bind _bjukebox (Variables|Default|GetbJukebox))
  (bind _pdaheist (Variables|/Game/Mods/HeistJukebox/HeistSoundtrackPersistentObject.HeistSoundtrackPersistentObject_C|GetPDAHeist _jukeboxpersistent))
  ;[1 1 1] Load values off of a save so I know if its fucky
  (bind _returnvalue (SaveGame|LoadGamefromSlot "VoidSave"))
  (bind _asbp_void_save (Utilities|Casting|CastToBP_VoidSave _returnvalue)
    (:then
      (Variables|Default|SetBannerPos (Variables|/Game/Mods/_TannerMod/VoidUIBanner/BP_VoidSave.BP_VoidSave_C|GetS_BannerPos _asbp_void_save))
      (Variables|Default|SetBannerScale (Variables|/Game/Mods/_TannerMod/VoidUIBanner/BP_VoidSave.BP_VoidSave_C|GetS_BannerScale _asbp_void_save))
      (Variables|Default|SetSettingsKey (Variables|/Game/Mods/_TannerMod/VoidUIBanner/BP_VoidSave.BP_VoidSave_C|GetS_SettingsKey _asbp_void_save))
      (Widget|Transform|SetRenderScale (Variables|/Game/Mods/_TannerMod/VoidUIBanner/WBP_VoidUIAssaultBanner.WBP_VoidUIAssaultBanner_C|GetAssNewMkp (stale Custom|OnActionPhasedEntered_Event_0 _returnvalue)) (Variables|Default|GetBannerScale))
      (Class|Widget|SetRenderTranslation (Variables|/Game/Mods/_TannerMod/VoidUIBanner/WBP_VoidUIAssaultBanner.WBP_VoidUIAssaultBanner_C|GetAssNewMkp (stale Custom|OnActionPhasedEntered_Event_0 _returnvalue)) (Variables|Default|GetBannerPos))
      ;[1 1 1] Track DebugShtik
      (if (.use (Utilities|Struct|Breaks_bpmdebug (Variables|/Game/Mods/_TannerMod/VoidUIBanner/BP_VoidSave.BP_VoidSave_C|GetS_Debug_BPMDebug _asbp_void_save)))
        (Default|AnBannerSetBlinkSpeed (stale Custom|OnActionPhasedEntered_Event_0 _returnvalue) (.values (Utilities|Struct|Breaks_bpmdebug (Variables|/Game/Mods/_TannerMod/VoidUIBanner/BP_VoidSave.BP_VoidSave_C|GetS_Debug_BPMDebug _asbp_void_save))))
        (bind _foundwidgets (Widget|GetAllWidgetsOfClass "/Game/Mods/_TannerMod/VoidUIBanner/WBP_VoidSettingsMkp.WBP_VoidSettingsMkp_C" false))
        (for _array_element _foundwidgets
          (Default|AnBannerSettingsSetBPMDebug _array_element (.values (Utilities|Struct|Breaks_bpmdebug (Variables|/Game/Mods/_TannerMod/VoidUIBanner/BP_VoidSave.BP_VoidSave_C|GetS_Debug_BPMDebug _asbp_void_save))) true))
        (else
          ;[0.2705 0.4125 0.04817] Track handler part 2 electric boogalo
          ;;[1 1 1] Compare if we have ost settings for that ak event
          (if _bjukebox
            (if (.ReturnValue (Utilities|Map|Find (Variables|Default|GetOstMap) (select _bjukebox (Variables|/Game/Mods/HeistJukebox/PDA_HeistSoundtrack.PDA_HeistSoundtrack_C|GetAudio%20Event _pdaheist) (Variables|/Script/Starbreeze.SBZWorldSettings|GetMusicEvent (stale _array_element_3))))) :!label _label
              (Default|AnBannerSetBlinkSpeed (stale Custom|OnActionPhasedEntered_Event_0 _returnvalue) (.Value (Utilities|Map|Find (Variables|Default|GetOstMap) (select _bjukebox (Variables|/Game/Mods/HeistJukebox/PDA_HeistSoundtrack.PDA_HeistSoundtrack_C|GetAudio%20Event _pdaheist) (Variables|/Script/Starbreeze.SBZWorldSettings|GetMusicEvent (stale _array_element_3))))))
              (bind _foundwidgets_2 (Widget|GetAllWidgetsOfClass "/Game/Mods/_TannerMod/VoidUIBanner/WBP_VoidSettingsMkp.WBP_VoidSettingsMkp_C" false))
              (for _array_element_2 _foundwidgets_2
                (Default|AnBannerSettingsSetBPMDebug _array_element_2 (.Value (Utilities|Map|Find (Variables|Default|GetOstMap) (select _bjukebox (Variables|/Game/Mods/HeistJukebox/PDA_HeistSoundtrack.PDA_HeistSoundtrack_C|GetAudio%20Event _pdaheist) (Variables|/Script/Starbreeze.SBZWorldSettings|GetMusicEvent (stale _array_element_3))))) true))
              (else
                (CallFunction|PrinttoModLoader (Utilities|String|Append "[AnBanner] Failed to find bpm entry for this track | " (select _bjukebox (Utilities|String|ToString(Text) (Variables|/Game/Mods/HeistJukebox/PDA_HeistSoundtrack.PDA_HeistSoundtrack_C|GetName _pdaheist)) (Utilities|GetDisplayName (Variables|/Script/Starbreeze.SBZWorldSettings|GetMusicEvent (stale _array_element_3))))))))
            (else
              (bind _outactors (Actor|GetAllActorsOfClass "/Script/Starbreeze.SBZWorldSettings"))
              (for _array_element_3 _outactors
                (goto _label)))))))
    (:CastFailed
      (CallFunction|PrinttoModLoader "[AnBanner] LoadGame on Update Cast Failed"))))

(event Custom|EventLeDebug
  ;[1 1 1] le giga secret debug button
  (Utilities|FlowControl|FlipFlop
    (:A
      (Widget|SetVisibility (Variables|/Game/Mods/_TannerMod/VoidUIBanner/WBP_VoidUIAssaultBanner.WBP_VoidUIAssaultBanner_C|GetDebugCanvas (stale Custom|OnActionPhasedEntered_Event_0 _returnvalue)) "Visible"))
    (:B
      (Widget|SetVisibility (Variables|/Game/Mods/_TannerMod/VoidUIBanner/WBP_VoidUIAssaultBanner.WBP_VoidUIAssaultBanner_C|GetDebugCanvas (stale Custom|OnActionPhasedEntered_Event_0 _returnvalue)) "Collapsed"))))

(event Custom|eventVoidBannerVisualUpdate
  (params (VisualBannerPos :type Vector%202D%20Structure) (VisualBannerScale :type Vector%202D%20Structure))
  (bind _jukeboxpersistent (Variables|Default|GetJukeboxPersistent))
  (bind _bjukebox (Variables|Default|GetbJukebox))
  (bind _pdaheist (Variables|/Game/Mods/HeistJukebox/HeistSoundtrackPersistentObject.HeistSoundtrackPersistentObject_C|GetPDAHeist _jukeboxpersistent))
  ;[1 1 1] Separate scroll box sliding so we dont save 1852852 times/second
  (Variables|Default|SetBannerPos VisualBannerPos)
  (Variables|Default|SetBannerScale VisualBannerScale)
  (Widget|Transform|SetRenderScale (Variables|/Game/Mods/_TannerMod/VoidUIBanner/WBP_VoidUIAssaultBanner.WBP_VoidUIAssaultBanner_C|GetAssNewMkp (stale Custom|OnActionPhasedEntered_Event_0 _returnvalue)) (Variables|Default|GetBannerScale))
  (Class|Widget|SetRenderTranslation (Variables|/Game/Mods/_TannerMod/VoidUIBanner/WBP_VoidUIAssaultBanner.WBP_VoidUIAssaultBanner_C|GetAssNewMkp (stale Custom|OnActionPhasedEntered_Event_0 _returnvalue)) (Variables|Default|GetBannerPos))
  ;[1 1 1] Track DebugShtik
  (if (.use (Utilities|Struct|Breaks_bpmdebug (Variables|/Game/Mods/_TannerMod/VoidUIBanner/BP_VoidSave.BP_VoidSave_C|GetS_Debug_BPMDebug (stale Custom|eventVoidBannerUpdate _asbp_void_save))))
    (Default|AnBannerSetBlinkSpeed (stale Custom|OnActionPhasedEntered_Event_0 _returnvalue) (.values (Utilities|Struct|Breaks_bpmdebug (Variables|/Game/Mods/_TannerMod/VoidUIBanner/BP_VoidSave.BP_VoidSave_C|GetS_Debug_BPMDebug (stale Custom|eventVoidBannerUpdate _asbp_void_save)))))
    (bind _foundwidgets (Widget|GetAllWidgetsOfClass "/Game/Mods/_TannerMod/VoidUIBanner/WBP_VoidSettingsMkp.WBP_VoidSettingsMkp_C" false))
    (for _array_element _foundwidgets
      (Default|AnBannerSettingsSetBPMDebug _array_element (.values (Utilities|Struct|Breaks_bpmdebug (Variables|/Game/Mods/_TannerMod/VoidUIBanner/BP_VoidSave.BP_VoidSave_C|GetS_Debug_BPMDebug (stale Custom|eventVoidBannerUpdate _asbp_void_save)))) true))
    (else
      ;[0.2705 0.4125 0.04817] Track handler part 2 electric boogalo
      ;;[1 1 1] Compare if we have ost settings for that ak event
      (if _bjukebox
        (if (.ReturnValue (Utilities|Map|Find (Variables|Default|GetOstMap) (select _bjukebox (Variables|/Game/Mods/HeistJukebox/PDA_HeistSoundtrack.PDA_HeistSoundtrack_C|GetAudio%20Event _pdaheist) (Variables|/Script/Starbreeze.SBZWorldSettings|GetMusicEvent (stale _array_element_3))))) :!label _label
          (Default|AnBannerSetBlinkSpeed (stale Custom|OnActionPhasedEntered_Event_0 _returnvalue) (.Value (Utilities|Map|Find (Variables|Default|GetOstMap) (select _bjukebox (Variables|/Game/Mods/HeistJukebox/PDA_HeistSoundtrack.PDA_HeistSoundtrack_C|GetAudio%20Event _pdaheist) (Variables|/Script/Starbreeze.SBZWorldSettings|GetMusicEvent (stale _array_element_3))))))
          (bind _foundwidgets_2 (Widget|GetAllWidgetsOfClass "/Game/Mods/_TannerMod/VoidUIBanner/WBP_VoidSettingsMkp.WBP_VoidSettingsMkp_C" false))
          (for _array_element_2 _foundwidgets_2
            (Default|AnBannerSettingsSetBPMDebug _array_element_2 (.Value (Utilities|Map|Find (Variables|Default|GetOstMap) (select _bjukebox (Variables|/Game/Mods/HeistJukebox/PDA_HeistSoundtrack.PDA_HeistSoundtrack_C|GetAudio%20Event _pdaheist) (Variables|/Script/Starbreeze.SBZWorldSettings|GetMusicEvent (stale _array_element_3))))) true))
          (else
            (CallFunction|PrinttoModLoader (Utilities|String|Append "[AnBanner] Failed to find bpm entry for this track | " (select _bjukebox (Utilities|String|ToString(Text) (Variables|/Game/Mods/HeistJukebox/PDA_HeistSoundtrack.PDA_HeistSoundtrack_C|GetName _pdaheist)) (Utilities|GetDisplayName (Variables|/Script/Starbreeze.SBZWorldSettings|GetMusicEvent (stale _array_element_3))))))))
        (else
          (bind _outactors (Actor|GetAllActorsOfClass "/Script/Starbreeze.SBZWorldSettings"))
          (for _array_element_3 _outactors
            (goto _label)))))))

(event Custom|OnActionPhasedEntered_Event_0
  (bind _jukeboxpersistent (Variables|Default|GetJukeboxPersistent))
  (bind _bjukebox (Variables|Default|GetbJukebox))
  (bind _pdaheist (Variables|/Game/Mods/HeistJukebox/HeistSoundtrackPersistentObject.HeistSoundtrackPersistentObject_C|GetPDAHeist _jukeboxpersistent))
  (bind _returnvalue (UserInterface|CreateWidget "/Game/Mods/_TannerMod/VoidUIBanner/WBP_VoidUIAssaultBanner.WBP_VoidUIAssaultBanner_C"))
  (UserInterface|Viewport|AddtoViewport _returnvalue 0)
  (Widget|Transform|SetRenderScale (Variables|/Game/Mods/_TannerMod/VoidUIBanner/WBP_VoidUIAssaultBanner.WBP_VoidUIAssaultBanner_C|GetAssNewMkp _returnvalue) (Variables|Default|GetBannerScale))
  (Class|Widget|SetRenderTranslation (Variables|/Game/Mods/_TannerMod/VoidUIBanner/WBP_VoidUIAssaultBanner.WBP_VoidUIAssaultBanner_C|GetAssNewMkp _returnvalue) (Variables|Default|GetBannerPos))
  ;[1 1 1] Track DebugShtik
  (if (.use (Utilities|Struct|Breaks_bpmdebug (Variables|/Game/Mods/_TannerMod/VoidUIBanner/BP_VoidSave.BP_VoidSave_C|GetS_Debug_BPMDebug (stale Custom|eventVoidBannerUpdate _asbp_void_save))))
    (Default|AnBannerSetBlinkSpeed _returnvalue (.values (Utilities|Struct|Breaks_bpmdebug (Variables|/Game/Mods/_TannerMod/VoidUIBanner/BP_VoidSave.BP_VoidSave_C|GetS_Debug_BPMDebug (stale Custom|eventVoidBannerUpdate _asbp_void_save)))))
    (bind _foundwidgets (Widget|GetAllWidgetsOfClass "/Game/Mods/_TannerMod/VoidUIBanner/WBP_VoidSettingsMkp.WBP_VoidSettingsMkp_C" false))
    (for _array_element _foundwidgets
      (Default|AnBannerSettingsSetBPMDebug _array_element (.values (Utilities|Struct|Breaks_bpmdebug (Variables|/Game/Mods/_TannerMod/VoidUIBanner/BP_VoidSave.BP_VoidSave_C|GetS_Debug_BPMDebug (stale Custom|eventVoidBannerUpdate _asbp_void_save)))) true))
    (else
      ;[0.2705 0.4125 0.04817] Track handler part 2 electric boogalo
      ;;[1 1 1] Compare if we have ost settings for that ak event
      (if _bjukebox
        (if (.ReturnValue (Utilities|Map|Find (Variables|Default|GetOstMap) (select _bjukebox (Variables|/Game/Mods/HeistJukebox/PDA_HeistSoundtrack.PDA_HeistSoundtrack_C|GetAudio%20Event _pdaheist) (Variables|/Script/Starbreeze.SBZWorldSettings|GetMusicEvent (stale _array_element_3))))) :!label _label
          (Default|AnBannerSetBlinkSpeed _returnvalue (.Value (Utilities|Map|Find (Variables|Default|GetOstMap) (select _bjukebox (Variables|/Game/Mods/HeistJukebox/PDA_HeistSoundtrack.PDA_HeistSoundtrack_C|GetAudio%20Event _pdaheist) (Variables|/Script/Starbreeze.SBZWorldSettings|GetMusicEvent (stale _array_element_3))))))
          (bind _foundwidgets_2 (Widget|GetAllWidgetsOfClass "/Game/Mods/_TannerMod/VoidUIBanner/WBP_VoidSettingsMkp.WBP_VoidSettingsMkp_C" false))
          (for _array_element_2 _foundwidgets_2
            (Default|AnBannerSettingsSetBPMDebug _array_element_2 (.Value (Utilities|Map|Find (Variables|Default|GetOstMap) (select _bjukebox (Variables|/Game/Mods/HeistJukebox/PDA_HeistSoundtrack.PDA_HeistSoundtrack_C|GetAudio%20Event _pdaheist) (Variables|/Script/Starbreeze.SBZWorldSettings|GetMusicEvent (stale _array_element_3))))) true))
          (else
            (CallFunction|PrinttoModLoader (Utilities|String|Append "[AnBanner] Failed to find bpm entry for this track | " (select _bjukebox (Utilities|String|ToString(Text) (Variables|/Game/Mods/HeistJukebox/PDA_HeistSoundtrack.PDA_HeistSoundtrack_C|GetName _pdaheist)) (Utilities|GetDisplayName (Variables|/Script/Starbreeze.SBZWorldSettings|GetMusicEvent (stale _array_element_3))))))))
        (else
          (bind _outactors (Actor|GetAllActorsOfClass "/Script/Starbreeze.SBZWorldSettings"))
          (for _array_element_3 _outactors
            (goto _label)))))))

(event EventBeginPlay
  (bind _returnvalue (Class|SBZPlayerLibrary|GetLocalPlayerController))
  (|CallParentFunction)
  (bind _returnvalue_2 (Class|SBZEventLibrary|GetGameEventBroker))
  (EventDispatchers|BindEventtoOnActionPhaseEntered _returnvalue_2 (delegate Custom|OnActionPhasedEntered_Event_0))
  (Utilities|FlowControl|Sequence
    (:then_0
      ;[1 1 1] Setting gui event binding bs
      (bind _returnvalue_3 (UserInterface|CreateWidget "/Game/Mods/_TannerMod/VoidUIBanner/WBP_VoidSettingsMkp.WBP_VoidSettingsMkp_C"))
      (UserInterface|Viewport|AddtoViewport _returnvalue_3 1)
      (EventDispatchers|BindEventtoEventVoidBannerUpdate _returnvalue_3 (EventDispatchers|CreateEvent :!event Custom|eventVoidBannerUpdate))
      (EventDispatchers|BindEventtoEventVoidBannerVisualUpdate _returnvalue_3 (EventDispatchers|CreateEvent :!event Custom|eventVoidBannerVisualUpdate))
      (EventDispatchers|BindEventtoLeDebug _returnvalue_3 (EventDispatchers|CreateEvent :!event Custom|EventLeDebug))
      ;[1 1 1] Visibility and mouse control for setting gui
      (Utilities|FlowControl|FlipFlop
        (:A
          (Widget|SetVisibility _returnvalue_3 "Collapsed")
          (Variables|/Script/Engine.PlayerController|SetbShowMouseCursor _returnvalue false)
          (Input|SetInputModeGameOnly _returnvalue))
        (:B
          (Widget|SetVisibility _returnvalue_3 "Visible")
          (Variables|/Script/Engine.PlayerController|SetbShowMouseCursor _returnvalue true)
          (Input|SetInputModeGameandUI _returnvalue _returnvalue_3 "DoNotLock" true))))
    (:then_1
      ;[1 1 1] Load pos when we have a settings gui
      (bind _returnvalue_4 (SaveGame|LoadGamefromSlot "VoidSave"))
      (bind _asbp_void_save (Utilities|Casting|CastToBP_VoidSave _returnvalue_4)
        (:then
          (Variables|Default|SetBannerPos (Variables|/Game/Mods/_TannerMod/VoidUIBanner/BP_VoidSave.BP_VoidSave_C|GetS_BannerPos _asbp_void_save))
          (Variables|Default|SetBannerScale (Variables|/Game/Mods/_TannerMod/VoidUIBanner/BP_VoidSave.BP_VoidSave_C|GetS_BannerScale _asbp_void_save))
          (Variables|Default|SetSettingsKey (Variables|/Game/Mods/_TannerMod/VoidUIBanner/BP_VoidSave.BP_VoidSave_C|GetS_SettingsKey _asbp_void_save)))
        (:CastFailed
          (CallFunction|PrinttoModLoader "[AnBanner] LoadGame on Start failed"))))
    (:then_2
      ;[0.6591 1 0.1188] Track speed handler
      (CallFunction|FindAssets "/Game/Mods/_TannerMod/VoidUIBanner/CTracks")
      ;;[1 1 1] Check if we have heist jukebox
      (bind _modloadermanagerinstance (CallFunction|GetModLoaderManager))
      (for _array_element (Variables|/Game/Mods/ModLoader/Blueprints/ModLoaderManager.ModLoaderManager_C|GetParsedModData _modloadermanagerinstance)
        (if (Utilities|Name|Equal(Name) (Variables|/Game/Mods/ModLoader/Blueprints/PDA_ModMeta.PDA_ModMeta_C|GetModID _array_element) "Heist_Jukebox")
          (Variables|Default|SetbJukebox true)
          (bind (_objectinstance _bfound) (CallFunction|FindPersistentModObjectbyClass "/Game/Mods/HeistJukebox/HeistSoundtrackPersistentObject.HeistSoundtrackPersistentObject_C"))
          (if _bfound
            (bind _asheist_soundtrack_persistent_object (Utilities|Casting|CastToHeistSoundtrackPersistentObject _objectinstance))
            (Variables|Default|SetJukeboxPersistent _asheist_soundtrack_persistent_object)
            (else
              (CallFunction|PrinttoModLoader "[AnBanner] Didn't Find jukebox persitent!"))))))))

(event EventTick
  (params (DeltaSeconds :type Float%20%28single-precision%29))
  (bind _returnvalue (Class|SBZPlayerLibrary|GetLocalPlayerController))
  ;[1 1 1] Visibility and mouse control for setting gui
  (if (Game|Player|WasInputKeyJustPressed _returnvalue (Variables|Default|GetSettingsKey))
    (Utilities|FlowControl|FlipFlop
      (:A
        (Widget|SetVisibility (stale EventBeginPlay _returnvalue_3) "Collapsed")
        (Variables|/Script/Engine.PlayerController|SetbShowMouseCursor _returnvalue false)
        (Input|SetInputModeGameOnly _returnvalue))
      (:B
        (Widget|SetVisibility (stale EventBeginPlay _returnvalue_3) "Visible")
        (Variables|/Script/Engine.PlayerController|SetbShowMouseCursor _returnvalue true)
        (Input|SetInputModeGameandUI _returnvalue (stale EventBeginPlay _returnvalue_3) "DoNotLock" true)))))

(fn ConstructionScript
  (|CallParentFunction))

(fn FindAssets
  (params (Folder :type String))
  (bind _returnvalue (Class|AssetRegistryHelpers|GetAssetRegistry))
  (bind _array (Utilities|Array|MakeArray Folder))
  (Class|AssetRegistry|ScanPathsSynchronous _returnvalue _array true)
  (for _array_element _array
    (bind _outassetdata (Class|AssetRegistry|GetAssetsbyPath _returnvalue (Utilities|String|StringToName _array_element) false false))
    (for _array_element_2 _outassetdata
      (bind _returnvalue_2 (Utilities|LoadAssetBlocking (Class|KismetSystemLibrary|ToSoftObjRef(SoftObjPath) (Utilities|MakeSoftObjectPath (Utilities|String|Replace (Class|KismetSystemLibrary|GetPathName (Class|AssetRegistryHelpers|GetAsset _array_element_2)) "." ".Default__")))))
      (bind _asda_ost_bpm (Utilities|Casting|CastToDA_OstBPM _returnvalue_2)
        (:then
          (Utilities|Map|Add (Variables|Default|GetOstMap) (Variables|/Game/Mods/_TannerMod/VoidUIBanner/DA_OstBPM.DA_OstBPM_C|GetAk%20Event _asda_ost_bpm) (Utilities|Struct|MakeOstStructure (Variables|/Game/Mods/_TannerMod/VoidUIBanner/DA_OstBPM.DA_OstBPM_C|GetBPM _asda_ost_bpm) (Variables|/Game/Mods/_TannerMod/VoidUIBanner/DA_OstBPM.DA_OstBPM_C|GetOffset _asda_ost_bpm) (Variables|/Game/Mods/_TannerMod/VoidUIBanner/DA_OstBPM.DA_OstBPM_C|GetMultiplier1 _asda_ost_bpm) (Variables|/Game/Mods/_TannerMod/VoidUIBanner/DA_OstBPM.DA_OstBPM_C|GetMultiplier2 _asda_ost_bpm) (Variables|/Game/Mods/_TannerMod/VoidUIBanner/DA_OstBPM.DA_OstBPM_C|GetMultiplier3 _asda_ost_bpm))))
        (:CastFailed
          (CallFunction|PrinttoModLoader (Utilities|String|Append "[AnBanner] Failed to cast asset, are you sure it's the correct type? | " (Utilities|GetDisplayName _returnvalue_2))))))
    (CallFunction|PrinttoModLoader "[AnBanner] Completed looking for assets")
    (return (Variables|Default|GetOstMap))))