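; Mod actor that swaps the CrimeNet heist selection screen for a custom contract selection UI.
; On BeginPlay it binds to visibility changes on the heist selection widgets, then creates the contract select widget and collapses the originals whenever one becomes visible.
; A refresh event resolves the heist banner soft reference, blocking-loading it if needed, and pushes the sprite into the contract confirm widgets via SSContractor.
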(event Custom|OnHeistSelection_0
  (params (InVisibility :type ESlateVisibility%20Enum :default "Visible"))
  (switch Utilities|FlowControl|Switch|SwitchonESlateVisibility InVisibility
    (:Visible
      (bind _returnvalue (UserInterface|CreateWidget "/Game/Mods/_TannerMod/LizHeistSelect/wbp_contractselect.wbp_contractselect_C"))
      (UserInterface|Viewport|AddtoViewport _returnvalue 1)
      (Widget|SetVisibility _returnvalue "Visible")
      (bind _foundwidgets (Widget|GetAllWidgetsOfClass "/Game/UI/Widgets/StateMachine/CrimeNet/WBP_SM_CrimeNetHeistSelection.WBP_SM_CrimeNetHeistSelection_C" false))
      (for _array_element _foundwidgets
        (Widget|SetVisibility _array_element "Collapsed")))))

(event Custom|requestRefresh
  (params (HeistData :type PD3%20Heist%20Data%20Asset%20Object%20Reference))
  (bind _foundwidgets (Widget|GetAllWidgetsOfClass "/Game/Mods/_TannerMod/LizHeistSelect/wbp_contractconfirm.wbp_contractconfirm_C" false))
  (for _array_element _foundwidgets
    (bind _returnvalue (Utilities|GetSprite (Variables|/Script/Starbreeze.PD3HeistDataAsset|GetHeistBannerImage HeistData)))
    (Rendering|Components|Sprite|SetSprite (Variables|Default|GetSS_Contractor) _returnvalue)
    (Variables|/Game/Mods/_TannerMod/LizHeistSelect/wbp_contractconfirm.wbp_contractconfirm_C|SetSS_Sprite _array_element (Variables|Default|GetSS_Contractor))
    (Variables|/Game/Mods/_TannerMod/LizHeistSelect/wbp_contractconfirm.wbp_contractconfirm_C|SetSprit _array_element _returnvalue)
    (Default|Refresh _array_element)))

(event EventBeginPlay
  (bind _foundwidgets (Widget|GetAllWidgetsOfClass "/Game/UI/Widgets/StateMachine/CrimeNet/WBP_SM_CrimeNetHeistSelection.WBP_SM_CrimeNetHeistSelection_C" false))
  (for _array_element _foundwidgets
    (bind _output_get (Variables|Default|SetHeistSelectionBase _array_element))
    (EventDispatchers|BindEventtoOnVisibilityChanged _output_get (delegate Custom|OnHeistSelection_0))))

(event Collision|EventActorBeginOverlap
  (params (OtherActor :type Actor%20Object%20Reference)))

(event EventTick
  (params (DeltaSeconds :type Float%20%28single-precision%29)))

(fn ConstructionScript
  (|CallParentFunction))