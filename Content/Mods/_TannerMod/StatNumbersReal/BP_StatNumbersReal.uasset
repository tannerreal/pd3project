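; BP_StatNumbersReal is a mod actor that puts a stat number widget on screen and provides damage logging.
; On BeginPlay it creates WBP_StatNumberWidget and adds it to the viewport.
; PrintDamage, with no caller in this Blueprint, prints a tagged line to the mod loader with a base/comp label, damage, distance divided by 100 and the FireData armor penetration.
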(event EventBeginPlay
  (|CallParentFunction)
  (bind _returnvalue (UserInterface|CreateWidget "/Game/Mods/_TannerMod/StatNumbersReal/WBP_StatNumberWidget.WBP_StatNumberWidget_C"))
  (UserInterface|Viewport|AddtoViewport _returnvalue 1))

(event Collision|EventActorBeginOverlap
  (params (OtherActor :type Actor%20Object%20Reference)))

(fn ConstructionScript
  (|CallParentFunction))