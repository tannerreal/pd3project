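; Mod actor in the txswapper folder that puts the Wbp_assmanager widget on screen and turns hotkeys into update calls.
; On BeginPlay it creates the widget and adds it to the viewport.
; Tick polls the first player controller for Slash and Period presses, calling UpdateMe with false or true respectively.
; The file does not show what responds to that call.
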(event EventBeginPlay
  (bind _returnvalue (UserInterface|CreateWidget "/Game/Mods/_TannerMod/txswapper/wbp_assmanager.wbp_assmanager_C"))
  (UserInterface|Viewport|AddtoViewport _returnvalue 1))

(event Collision|EventActorBeginOverlap
  (params (OtherActor :type Actor%20Object%20Reference)))

(event EventTick
  (params (DeltaSeconds :type Float%20%28single-precision%29))
  (Utilities|FlowControl|Sequence
    (:then_0
      (if (Game|Player|WasInputKeyJustPressed (Game|GetPlayerController 0) "Slash")
        (Default|CallUpdateMe false)))
    (:then_1
      (if (Game|Player|WasInputKeyJustPressed (Game|GetPlayerController 0) "Period")
        (Default|CallUpdateMe true)))))

(fn ConstructionScript
  (|CallParentFunction))