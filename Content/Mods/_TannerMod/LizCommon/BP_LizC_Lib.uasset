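; Shared helper Blueprint for the LizC mod that finds and loads assets synchronously.
; FindAssets scans folders non-recursively through the asset registry and blocking-loads each asset, optionally rewriting paths to target class default objects.
; LoadAsset resolves or blocking-loads a soft reference and returns a validity flag, while LoadAssetVerbose also logs failures to the mod loader.
; IsModLevel's "/Mods" path check is left unwired.
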(event EventBeginPlay)

(event Collision|EventActorBeginOverlap
  (params (OtherActor :type Actor%20Object%20Reference)))

(event EventTick
  (params (DeltaSeconds :type Float%20%28single-precision%29)))

(fn ConstructionScript
  (|CallParentFunction))

(fn FindAssets
  (params (Directories :type Array%20of%20Strings) (Append%20Default :type Boolean))
  (bind _returnvalue (Class|AssetRegistryHelpers|GetAssetRegistry))
  (bind _tmp_objarray (LocalVariables|Gettmp_objarray))
  (Class|AssetRegistry|ScanPathsSynchronous _returnvalue Directories false)
  (for _array_element Directories
    (bind _outassetdata (Class|AssetRegistry|GetAssetsbyPath _returnvalue (Utilities|String|StringToName _array_element) false false))
    (for _array_element_2 _outassetdata
      (bind _returnvalue_2 (Utilities|LoadAssetBlocking (Class|KismetSystemLibrary|ToSoftObjRef(SoftObjPath) (Utilities|MakeSoftObjectPath (Utilities|String|Replace (Class|KismetSystemLibrary|GetPathName (Class|AssetRegistryHelpers|GetAsset _array_element_2)) "." (select Append%20Default ".Default__" "."))))))
      (Utilities|Array|Add _tmp_objarray _returnvalue_2))
    (CallFunction|PrinttoModLoader "[LizLib] Finished finding assets in this folder"))
  (return _tmp_objarray (Utilities|Array|Length _tmp_objarray)))

(fn LoadAsset
  (params (Asset :type Object%20Soft%20Object%20Reference))
  (bind _output (Utilities|ResolveSoftReference Asset))
  (Utilities|IsValid _output
    (:Is%20Valid
      (return _output true))
    (:Is%20Not%20Valid
      (bind _returnvalue (Utilities|LoadAssetBlocking Asset))
      (Utilities|IsValid _returnvalue
        (:Is%20Valid
          (return _returnvalue true))
        (:Is%20Not%20Valid
          (return 0 false))))))

(fn LoadAssetVerbose
  (params (Asset :type Object%20Soft%20Object%20Reference))
  (bind _output (Utilities|ResolveSoftReference Asset))
  (Utilities|IsValid _output
    (:Is%20Valid
      (return _output true))
    (:Is%20Not%20Valid
      (bind _returnvalue (Utilities|LoadAssetBlocking Asset))
      (Utilities|IsValid _returnvalue
        (:Is%20Valid
          (return _returnvalue true))
        (:Is%20Not%20Valid
          (CallFunction|PrinttoModLoader (Utilities|String|ToString(Text) (Utilities|Text|FormatText "[LizLib] Failed to load a soft asset:  
> Soft: {Soft} 
> Resolved: {Reso} 
> Loaded: {Load}" (Utilities|ToString(SoftObjectReference) Asset) _output _returnvalue)))
          (return 0 false))))))

(fn IsModLevel
  (params (LevelPath :type Soft%20Object%20Path%20Structure)))