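; Mod actor for HeistJukebox that lets the player pick heist music in the pre-planning lobby.
; On BeginPlay it finds the persistent soundtrack object, restores its index, resets its choice to the first track and scans the mod's Music folder for soundtrack data assets via the Asset Registry.
; After pre-match loading it shows a selector widget; arrows cycle with wraparound and save the choice to that object, while Random toggles its random-song flag.
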(event Custom|EventOnPreMatchAsyncLoadingDone_0
  ;[0.5462 1 0.5603] Spawn Soundtrack selector widget once preplanning lobby is loaded
  (bind _returnvalue (UserInterface|CreateWidget "/Game/Mods/HeistJukebox/WBP_SoundtrackSelector-OLD.WBP_SoundtrackSelector-OLD_C"))
  (bind _output_get (Variables|Default|SetSoundtrack%20Selector%20Widget _returnvalue))
  (bind _pdaheistsoundtrack (CallFunction|GetCurrentPDA (Variables|Default|GetIndex)))
  (Default|SetWidgetText _output_get (Variables|/Game/Mods/HeistJukebox/PDA_HeistSoundtrack.PDA_HeistSoundtrack_C|GetName _pdaheistsoundtrack))
  (UserInterface|Viewport|AddtoViewport (Variables|Default|GetSoundtrack%20Selector%20Widget) 9999)
  (EventDispatchers|BindEventtoOnClicked (Variables|/Game/Mods/HeistJukebox/WBP_SoundtrackSelector-OLD.WBP_SoundtrackSelector-OLD_C|GetButton_LeftArrow (Variables|Default|GetSoundtrack%20Selector%20Widget)) (EventDispatchers|CreateEvent :!event Custom|EventOnLeftButtonClicked_0))
  (EventDispatchers|BindEventtoOnClicked (Variables|/Game/Mods/HeistJukebox/WBP_SoundtrackSelector-OLD.WBP_SoundtrackSelector-OLD_C|GetButton_RightArrow (Variables|Default|GetSoundtrack%20Selector%20Widget)) (EventDispatchers|CreateEvent :!event Custom|EventOnRightButtonClicked_0))
  (EventDispatchers|BindEventtoOnClicked (Variables|/Game/Mods/HeistJukebox/WBP_SoundtrackSelector-OLD.WBP_SoundtrackSelector-OLD_C|GetButton_Random (Variables|Default|GetSoundtrack%20Selector%20Widget)) (EventDispatchers|CreateEvent :!event Custom|EventOnRandomButtonClicked_0)))

(event Custom|EventOnRightButtonClicked_0
  (bind _as_heist_soundtrack_persistent_object (Variables|Default|GetAs%20Heist%20Soundtrack%20Persistent%20Object))
  ;[0.3733 0.8389 1] Handle changing soundtrack from button click
  (bind _result (Math|Integer|IncrementInt (Variables|Default|GetIndex))
    (:%20%20
      (if (== _result (Utilities|Array|Length (Variables|Default|GetPDAHeistSoundtrackarray)))
        (Variables|Default|SetIndex 0))
      (bind _pdaheistsoundtrack (CallFunction|GetCurrentPDA (Variables|Default|GetIndex)))
      (Default|SetWidgetText (Variables|Default|GetSoundtrack%20Selector%20Widget) (Variables|/Game/Mods/HeistJukebox/PDA_HeistSoundtrack.PDA_HeistSoundtrack_C|GetName _pdaheistsoundtrack))
      (Variables|/Game/Mods/HeistJukebox/HeistSoundtrackPersistentObject.HeistSoundtrackPersistentObject_C|SetPDAHeist _as_heist_soundtrack_persistent_object _pdaheistsoundtrack)
      (Variables|/Game/Mods/HeistJukebox/HeistSoundtrackPersistentObject.HeistSoundtrackPersistentObject_C|SetIndex _as_heist_soundtrack_persistent_object (Variables|Default|GetIndex)))))

(event Custom|EventOnLeftButtonClicked_0
  (bind _as_heist_soundtrack_persistent_object (Variables|Default|GetAs%20Heist%20Soundtrack%20Persistent%20Object))
  ;[0.3733 0.8389 1] Handle changing soundtrack from button click
  (bind _result (Math|Integer|DecrementInt (Variables|Default|GetIndex))
    (:%20%20
      (if (== _result -1)
        (Variables|Default|SetIndex (Utilities|Array|LastIndex (Variables|Default|GetPDAHeistSoundtrackarray))))
      (bind _pdaheistsoundtrack (CallFunction|GetCurrentPDA (Variables|Default|GetIndex)))
      (Default|SetWidgetText (Variables|Default|GetSoundtrack%20Selector%20Widget) (Variables|/Game/Mods/HeistJukebox/PDA_HeistSoundtrack.PDA_HeistSoundtrack_C|GetName _pdaheistsoundtrack))
      (Variables|/Game/Mods/HeistJukebox/HeistSoundtrackPersistentObject.HeistSoundtrackPersistentObject_C|SetPDAHeist _as_heist_soundtrack_persistent_object _pdaheistsoundtrack)
      (Variables|/Game/Mods/HeistJukebox/HeistSoundtrackPersistentObject.HeistSoundtrackPersistentObject_C|SetIndex _as_heist_soundtrack_persistent_object (Variables|Default|GetIndex)))))

(event Custom|EventOnRandomButtonClicked_0
  (bind _as_heist_soundtrack_persistent_object (Variables|Default|GetAs%20Heist%20Soundtrack%20Persistent%20Object))
  (if (Variables|/Game/Mods/HeistJukebox/HeistSoundtrackPersistentObject.HeistSoundtrackPersistentObject_C|GetrandomSong _as_heist_soundtrack_persistent_object)
    (Variables|/Game/Mods/HeistJukebox/HeistSoundtrackPersistentObject.HeistSoundtrackPersistentObject_C|SetrandomSong _as_heist_soundtrack_persistent_object false)
    (else
      (Variables|/Game/Mods/HeistJukebox/HeistSoundtrackPersistentObject.HeistSoundtrackPersistentObject_C|SetrandomSong _as_heist_soundtrack_persistent_object true))))

(event EventBeginPlay
  ;[1 0.4324 0.837] Spawn Actor, and bind event
  (|CallParentFunction)
  (bind _objectinstance (CallFunction|FindPersistentModObjectbyClass "/Game/Mods/HeistJukebox/HeistSoundtrackPersistentObject.HeistSoundtrackPersistentObject_C"))
  (bind _asheist_soundtrack_persistent_object (Utilities|Casting|CastToHeistSoundtrackPersistentObject _objectinstance)
    (:then
      (bind _output_get (Variables|Default|SetAs%20Heist%20Soundtrack%20Persistent%20Object _asheist_soundtrack_persistent_object))
      (Variables|Default|SetIndex (Variables|/Game/Mods/HeistJukebox/HeistSoundtrackPersistentObject.HeistSoundtrackPersistentObject_C|GetIndex _output_get))
      (bind _returnvalue (Class|SBZEventLibrary|GetGameEventBroker))
      (Variables|Default|SetGame%20Event%20Broker _returnvalue)
      (CallFunction|LoadAllPossibleSoundtracks)
      (CallFunction|SetInitialPDAHeist)
      (EventDispatchers|BindEventtoOnPreMatchAsyncLoadingDone (Variables|Default|GetGame%20Event%20Broker) (EventDispatchers|CreateEvent :!event Custom|EventOnPreMatchAsyncLoadingDone_0)))
    (:CastFailed
      (CallFunction|PrinttoModLoader "FAILED TO FIND HEIST SOUNDTRACK OBJECT"))))

(fn ConstructionScript
  (|CallParentFunction))

(fn CreateHeistSoundtrackArray
  (return (Utilities|Array|MakeArray (Utilities|Struct|MakeHeistSoundtrackStructure "No Rest For The Wicked" "/Game/WWiseAudio/Events/Music/Heists/MusicHeist_03_BranchBank.MusicHeist_03_BranchBank") (Utilities|Struct|MakeHeistSoundtrackStructure "Road Rage" "/Game/WWiseAudio/Events/Music/Heists/MusicHeist_04_ArmoredTransport.MusicHeist_04_ArmoredTransport") (Utilities|Struct|MakeHeistSoundtrackStructure "Dirty Ice" "/Game/WWiseAudio/Events/Music/Heists/MusicHeist_02_JewelryStore.MusicHeist_02_JewelryStore") (Utilities|Struct|MakeHeistSoundtrackStructure "Rock The Cradle" "/Game/WWiseAudio/Events/Music/Heists/MusicHeist_08_Nightclub.MusicHeist_08_Nightclub") (Utilities|Struct|MakeHeistSoundtrackStructure "Under The Surphaze" "/Game/WWiseAudio/Events/Music/Heists/MusicHeist_07_ArtGallery.MusicHeist_07_ArtGallery") (Utilities|Struct|MakeHeistSoundtrackStructure "Gold & Sharke" "/Game/WWiseAudio/Events/Music/Heists/MusicHeist_01_FirstPlayable.MusicHeist_01_FirstPlayable") (Utilities|Struct|MakeHeistSoundtrackStructure "99 Boxes" "/Game/WWiseAudio/Events/Music/Heists/MusicHeist_05_CargoDocks.MusicHeist_05_CargoDocks") (Utilities|Struct|MakeHeistSoundtrackStructure "Touch The Sky" "/Game/WWiseAudio/Events/Music/Heists/MusicHeist_06_Penthouse.MusicHeist_06_Penthouse"))))

(fn GetCurrentSoundtrackChoice
  (params (Index :type Integer))
  (return (Utilities|Array|Get(acopy) (Variables|Default|GetHeistSoundtrackArray) Index)))

(fn LoadAllPossibleSoundtracks
  (bind _returnvalue (Class|AssetRegistryHelpers|GetAssetRegistry))
  (Class|AssetRegistry|ScanPathsSynchronous _returnvalue (Utilities|Array|MakeArray "/Game/Mods/HeistJukebox/Music") false)
  (bind _outassetdata (Class|AssetRegistry|GetAssets _returnvalue (Utilities|MakeARFilter 0 (Utilities|Array|MakeArray "/Game/Mods/HeistJukebox/Music") 0 (Utilities|Array|MakeArray "BlueprintGeneratedClass") 0 true true)))
  (for _array_element _outassetdata
    (bind _returnvalue_2 (Utilities|LoadAssetBlocking (Class|KismetSystemLibrary|ToSoftObjRef(SoftObjPath) (Utilities|MakeSoftObjectPath (Utilities|String|Replace (Class|KismetSystemLibrary|GetPathName (Class|AssetRegistryHelpers|GetAsset _array_element)) "." ".Default__")))))
    (bind _aspda_heist_soundtrack (Utilities|Casting|CastToPDA_HeistSoundtrack _returnvalue_2)
      (:then
        (Utilities|Array|AddUnique (Variables|Default|GetPDAHeistSoundtrackarray) _aspda_heist_soundtrack))
      (:CastFailed
        (CallFunction|PrinttoModLoader "FAILED TO CAST ASSET!!")))))

(fn GetCurrentPDA
  (params (Index :type Integer))
  (return (Utilities|Array|Get(acopy) (Variables|Default|GetPDAHeistSoundtrackarray) Index)))

(fn SetInitialPDAHeist
  (Variables|/Game/Mods/HeistJukebox/HeistSoundtrackPersistentObject.HeistSoundtrackPersistentObject_C|SetPDAHeist (Variables|Default|GetAs%20Heist%20Soundtrack%20Persistent%20Object) (Utilities|Array|Get(acopy) (Variables|Default|GetPDAHeistSoundtrackarray))))