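; Heist Jukebox mod Blueprint that replaces the heist music with the soundtrack stored in the persistent mod object.
; On BeginPlay, a pending random request scans the mod's Music folder, stores a random pick in that object and clears the flag.
; LoadSongs finds Blueprint classes through the Asset Registry and loads their Default__ objects as soundtrack data.
; HeistOnly tracks start when the heist goes loud; others play immediately.
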(event Custom|EventOnHeistGoneLoud_0
  (bind _returnvalue (Class|SBZMusicManager|GetMusicManager))
  (Class|SBZMusicManager|StopMusic _returnvalue)
  (Class|SBZMusicManager|PlayMusic _returnvalue (Variables|/Game/Mods/HeistJukebox/PDA_HeistSoundtrack.PDA_HeistSoundtrack_C|GetAudio%20Event (Variables|/Game/Mods/HeistJukebox/HeistSoundtrackPersistentObject.HeistSoundtrackPersistentObject_C|GetPDAHeist (Variables|Default|GetAs%20Heist%20Soundtrack%20Persistent%20Object))) false))

(event EventBeginPlay
  (bind _returnvalue (Class|SBZMusicManager|GetMusicManager))
  (bind _objectinstance (CallFunction|FindPersistentModObjectbyClass "/Game/Mods/HeistJukebox/HeistSoundtrackPersistentObject.HeistSoundtrackPersistentObject_C"))
  (bind _asheist_soundtrack_persistent_object (Utilities|Casting|CastToHeistSoundtrackPersistentObject _objectinstance)
    (:then
      (Variables|Default|SetAs%20Heist%20Soundtrack%20Persistent%20Object _asheist_soundtrack_persistent_object)
      (if (Variables|/Game/Mods/HeistJukebox/HeistSoundtrackPersistentObject.HeistSoundtrackPersistentObject_C|GetrandomSong (Variables|Default|GetAs%20Heist%20Soundtrack%20Persistent%20Object))
        (CallFunction|LoadSongs)
        (Variables|/Game/Mods/HeistJukebox/HeistSoundtrackPersistentObject.HeistSoundtrackPersistentObject_C|SetPDAHeist (Variables|Default|GetAs%20Heist%20Soundtrack%20Persistent%20Object) (.OutItem (Utilities|Array|Random (Variables|Default|GetPDAHeistSoundtrackarray))))
        (Variables|/Game/Mods/HeistJukebox/HeistSoundtrackPersistentObject.HeistSoundtrackPersistentObject_C|SetrandomSong (Variables|Default|GetAs%20Heist%20Soundtrack%20Persistent%20Object) false))
      (if (Variables|/Game/Mods/HeistJukebox/PDA_HeistSoundtrack.PDA_HeistSoundtrack_C|GetHeist%20Only (Variables|/Game/Mods/HeistJukebox/HeistSoundtrackPersistentObject.HeistSoundtrackPersistentObject_C|GetPDAHeist (Variables|Default|GetAs%20Heist%20Soundtrack%20Persistent%20Object)))
        (bind _returnvalue_2 (Class|SBZEventLibrary|GetGameEventBroker))
        (EventDispatchers|BindEventtoOnHeistGoneLoud _returnvalue_2 (EventDispatchers|CreateEvent :!event Custom|EventOnHeistGoneLoud_0))
        (else
          (Class|SBZMusicManager|StopMusic _returnvalue)
          (Class|SBZMusicManager|PlayMusic _returnvalue (Variables|/Game/Mods/HeistJukebox/PDA_HeistSoundtrack.PDA_HeistSoundtrack_C|GetAudio%20Event (Variables|/Game/Mods/HeistJukebox/HeistSoundtrackPersistentObject.HeistSoundtrackPersistentObject_C|GetPDAHeist (Variables|Default|GetAs%20Heist%20Soundtrack%20Persistent%20Object))) false))))
    (:CastFailed
      (CallFunction|PrinttoModLoader "FAILED TO FIND PERSISTENT MOD OBJECT ON HEIST"))))

(fn ConstructionScript
  (|CallParentFunction))

(fn LoadSongs
  (bind _returnvalue (Class|AssetRegistryHelpers|GetAssetRegistry))
  (Class|AssetRegistry|ScanPathsSynchronous _returnvalue (Utilities|Array|MakeArray "/Game/Mods/HeistJukebox/Music") false)
  (bind _outassetdata (Class|AssetRegistry|GetAssets _returnvalue (Utilities|MakeARFilter 0 (Utilities|Array|MakeArray "/Game/Mods/HeistJukebox/Music") 0 (Utilities|Array|MakeArray "BlueprintGeneratedClass") 0 true true)))
  (for _array_element _outassetdata
    (bind _returnvalue_2 (Utilities|LoadAssetBlocking (Class|KismetSystemLibrary|ToSoftObjRef(SoftObjPath) (Utilities|MakeSoftObjectPath (Utilities|String|Replace (Class|KismetSystemLibrary|GetPathName (Class|AssetRegistryHelpers|GetAsset _array_element)) "." ".Default__")))))
    (bind _aspda_heist_soundtrack (Utilities|Casting|CastToPDA_HeistSoundtrack _returnvalue_2)
      (:then
        (Utilities|Array|AddUnique (Variables|Default|GetPDAHeistSoundtrackarray) _aspda_heist_soundtrack))
      (:CastFailed
        (CallFunction|PrinttoModLoader "FAILED TO CAST ASSET!!")))))