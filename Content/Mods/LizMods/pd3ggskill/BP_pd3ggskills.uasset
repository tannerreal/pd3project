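; Mod Blueprint that decodes pd3.gg skill build links against the game's skills menu and logs the result; equipping is only unwired stubs.
; On BeginPlay it caches the skills menu widget and adds its own widget to the viewport with a back-reference.
; The parser maps letters to skill line indices, uppercase meaning aced, and digits to skills, then checks earned points before logging names.
; A second event dumps all skill lines and skills with progress.
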(event Custom|pd3_printString
  (params (SourceString :type String))
  (bind _returnvalue (Utilities|String|Replace SourceString "https://pd3.gg/skills?s="))
  (bind _returnvalue_2 (Class|SBZSkillManager|GetSkillManager))
  (bind _tmp_skillmap (Variables|Default|Gettmp_skillMap))
  (bind _returnvalue_3 (Class|SBZSkillManager|GetEarnedSkillPoints _returnvalue_2))
  ;[1 1 1] String conversion
  (CallFunction|PrinttoModLoader (Utilities|String|Append "[pd3ggskills] " _returnvalue))
  (Utilities|Map|Clear (Variables|Default|Gettmp_skillMap))
  (Variables|Default|Settmp_lastSkillLineID 0)
  (Variables|Default|Settmp_skillStringArray "")
  (Variables|Default|Settmp_skillAmmount 0)
  (for _array_element (Utilities|String|GetCharacterArrayfromString _returnvalue)
    (if (Class|KismetStringLibrary|IsNumeric _array_element)
      (bind _output_get (Variables|Default|Settmp_skillStringArray (Utilities|String|Append (Variables|Default|Gettmp_skillStringArray) (select (Utilities|Enum|Equal(Enum) _array_element "1") (select (>= (Utilities|String|FindSubstring (Variables|Default|Gettmp_skillStringArray) "01") 0) "" "0") _array_element))))
      (Utilities|Map|Add (Variables|Default|Gettmp_skillMap) (Variables|Default|Gettmp_lastSkillLineID) _output_get)
      (else
        (bind _output_get_2 (Variables|Default|Settmp_lastSkillLineID (Math|Float|Truncate (Math|Float|MapRangeClamped (Math|Conversions|ToFloat(Integer) (Utilities|String|GetCharacterasNumber (Utilities|String|ToLower _array_element))) 97.0 122.0 0.0 25.0))))
        (bind _output_get_3 (Variables|Default|Settmp_skillStringArray (select (Utilities|Enum|Equal(Enum) (Utilities|String|ToLower _array_element) _array_element) "" "01")))
        (Utilities|Map|Add (Variables|Default|Gettmp_skillMap) _output_get_2 _output_get_3)))
    (Variables|Default|Settmp_skillAmmount (+ (Variables|Default|Gettmp_skillAmmount) 1)))
  ;[1 1 1] check if we have enough skill points
  (if (< _returnvalue_3 (Variables|Default|Gettmp_skillAmmount))
    (CallFunction|PrinttoModLoader (Utilities|String|ToString(Text) (Utilities|Text|FormatText "[pd3ggskills] You have less skill points than needed({has}/{needs})" _returnvalue_3 (Variables|Default|Gettmp_skillAmmount))))
    (else
      ;[1 1 1] Get all skill lines
      (bind _keys (Utilities|Map|Keys _tmp_skillmap))
      (for _array_element_2 _keys
        (CallFunction|PrinttoModLoader (Utilities|String|ToString(Text) (Utilities|Text|FormatText "[pd3ggskills] SkillLineId: {skid} Skills: {skstr}" _array_element_2 (.Value (Utilities|Map|Find _tmp_skillmap _array_element_2)))))
        ;[1 1 1] Find skills in skill lines that need equipping
        (for (_array_element_3 _array_index) (Utilities|String|GetCharacterArrayfromString (.Value (Utilities|Map|Find _tmp_skillmap _array_element_2)))
          (CallFunction|PrinttoModLoader (Utilities|String|ToString(Text) (Utilities|Text|FormatText "[pd3ggskills] SkillLine: {skl}({sklid}) Skill: {sk}({skid})" (Variables|/Script/Starbreeze.SBZInventoryBaseData|GetDisplayName (Variables|/Script/Starbreeze.SBZSkillLine|GetSkillLineData (Utilities|Array|Get(acopy) (Variables|/Game/UI/Widgets/StateMachine/Loadout/Skills/WBP_UI_Skills_Menu.WBP_UI_Skills_Menu_C|GetSkillLines (Variables|Default|GetSkillWidget)) _array_element_2))) _array_element_2 (Variables|/Script/Starbreeze.SBZInventoryBaseData|GetDisplayName (Variables|/Script/Starbreeze.SBZSkill|GetSkillData (Utilities|Array|Get(acopy) (Variables|/Script/Starbreeze.SBZSkillLine|GetSkills (Utilities|Array|Get(acopy) (Variables|/Game/UI/Widgets/StateMachine/Loadout/Skills/WBP_UI_Skills_Menu.WBP_UI_Skills_Menu_C|GetSkillLines (Variables|Default|GetSkillWidget)) _array_element_2)) (Math|Conversions|ToInteger(Byte) _array_element_3)))) _array_index))))))))

(event Custom|pd3_PrintSkills
  (for (_array_element _array_index) (Variables|/Game/UI/Widgets/StateMachine/Loadout/Skills/WBP_UI_Skills_Menu.WBP_UI_Skills_Menu_C|GetSkillLines (Variables|Default|GetSkillWidget))
    (CallFunction|PrinttoModLoader (Utilities|String|ToString(Text) (Utilities|Text|FormatText "[pd3ggskills] Skill line {skl}({id})[{research}] has the following skills:" (Variables|/Script/Starbreeze.SBZInventoryBaseData|GetDisplayName (Variables|/Script/Starbreeze.SBZSkillLine|GetSkillLineData _array_element)) _array_index (Variables|/Script/Starbreeze.SBZSkillLine|GetResearchPercentage _array_element))))
    (for (_array_element_2 _array_index_2) (Variables|/Script/Starbreeze.SBZSkillLine|GetSkills _array_element)
      (CallFunction|PrinttoModLoader (Utilities|String|ToString(Text) (Utilities|Text|FormatText "[pd3ggskills] >Skill line {skl}/Skill:{sk}({id})[{research}]" (Variables|/Script/Starbreeze.SBZInventoryBaseData|GetDisplayName (Variables|/Script/Starbreeze.SBZSkillLine|GetSkillLineData _array_element)) (Variables|/Script/Starbreeze.SBZInventoryBaseData|GetDisplayName (Variables|/Script/Starbreeze.SBZSkill|GetSkillData _array_element_2)) _array_index_2 (Variables|/Script/Starbreeze.SBZSkill|GetProgressPercentage _array_element_2)))))))

(event EventBeginPlay
  (bind _foundwidgets (Widget|GetAllWidgetsOfClass "/Game/UI/Widgets/StateMachine/Loadout/Skills/WBP_UI_Skills_Menu.WBP_UI_Skills_Menu_C" false))
  (for _array_element _foundwidgets
    (Variables|Default|SetSkillWidget _array_element)
    (bind _returnvalue (UserInterface|CreateWidget "/Game/Mods/LizMods/pd3ggskill/WBP_pd3ggskillWidget.WBP_pd3ggskillWidget_C"))
    (UserInterface|Viewport|AddtoViewport _returnvalue 1)
    (Variables|/Game/Mods/LizMods/pd3ggskill/WBP_pd3ggskillWidget.WBP_pd3ggskillWidget_C|SetMainBP _returnvalue self)))

(fn ConstructionScript
  (|CallParentFunction))